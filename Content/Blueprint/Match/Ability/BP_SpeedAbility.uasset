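; Match ability Blueprint that temporarily doubles the walk speed of its Hitter character.
; AuthUse multiplies the Hitter's CharacterMovement MaxWalkSpeed and starts a one-shot timer lasting Duration.
; AuthTimerEnd divides the current speed by the same factor rather than restoring a cached value, so overlapping uses compound.
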(event Custom|Auth%20Timer%20End
  (bind _hitter (Variables|Default|GetHitter))
  (bind _charactermovement (Variables|/Script/Engine.Character|GetCharacterMovement _hitter))
  (Variables|/Script/Engine.CharacterMovementComponent|SetMaxWalkSpeed _charactermovement (/ (Variables|/Script/Engine.CharacterMovementComponent|GetMaxWalkSpeed _charactermovement) 2.0)))

(event EventAuthUse
  (bind _hitter (Variables|Default|GetHitter))
  (bind _charactermovement (Variables|/Script/Engine.Character|GetCharacterMovement _hitter))
  (Variables|/Script/Engine.CharacterMovementComponent|SetMaxWalkSpeed _charactermovement (* (Variables|/Script/Engine.CharacterMovementComponent|GetMaxWalkSpeed _charactermovement) 2.0))
  (Utilities|Time|SetTimerbyEvent (delegate Custom|Auth%20Timer%20End) (Variables|Default|GetDuration)))

(fn ConstructionScript
  (|CallParentFunction))